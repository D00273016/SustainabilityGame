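; Base VR button Blueprint that a player presses by touching it with a VRPawn, apparently to purchase a dress.
; Begin and end overlaps on the button collision trigger interact and release, which toggle the button visuals.
; Pressing broadcasts the purchase dispatcher with its dress reference, then calls ButtonPressed, an empty event meant for child overrides or dispatcher bindings.
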(event `self.OnPlayerInteract`
  (params (HitResult :type "HitResult Structure"))
  ; Press the button when the player interacts
  (`self.OnPurchaseButtonPressed` (`self.BP_Dress`))
  (`self.ButtonPressed`)
  (`self.UpdateButtonVisuals` true))

(event `self.OnPlayerInteractRelease`
  ; Press the button when the player interacts
  (`self.UpdateButtonVisuals` false))

(event `ButtonPressed`
  ; Overwrite these in child blueprint or bind to event dispatcher depending on your requirements.
)

(event `self.ButtonCollision.OnComponentBeginOverlap`
  (params (OverlappedComponent :type "PrimitiveComponent Object Reference") (OtherActor :type "Actor Object Reference") (OtherComp :type "PrimitiveComponent Object Reference") (OtherBodyIndex :type Integer) (bFromSweep :type Boolean) (SweepResult :type "HitResult Structure (by ref)"))
  (cast `/Game/VRTemplate/Blueprints/VRPawn` OtherActor)
  (`/Game/Global/Blueprints/Interactive/BPI_PlayerInteraction.OnPlayerInteract` (struct)))

(event `self.ButtonCollision.OnComponentEndOverlap`
  (params (OverlappedComponent :type "PrimitiveComponent Object Reference") (OtherActor :type "Actor Object Reference") (OtherComp :type "PrimitiveComponent Object Reference") (OtherBodyIndex :type Integer))
  (cast `/Game/VRTemplate/Blueprints/VRPawn` OtherActor)
  (`/Game/Global/Blueprints/Interactive/BPI_PlayerInteraction.OnPlayerInteractRelease`))

(fn `UserConstructionScript`
  (`parent.UserConstructionScript`))