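; Shop music zone that plays a 2D sound while a VRPawn is inside its Box volume.
; On begin overlap it spawns the sound at boosted volume and stores the audio component, unless that component is already playing.
; On end overlap it calls HandleShopExit for any actor, then, for a VRPawn, silences and stops the playing component immediately.
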(event `self.Box.OnComponentBeginOverlap`
  (params (OverlappedComponent :type "PrimitiveComponent Object Reference") (OtherActor :type "Actor Object Reference") (OtherComp :type "PrimitiveComponent Object Reference") (OtherBodyIndex :type Integer) (bFromSweep :type Boolean) (SweepResult :type "HitResult Structure (by ref)"))
  (cast `/Game/VRTemplate/Blueprints/VRPawn` OtherActor)
  (if (not (`AudioComponent.IsPlaying` (`self.ShopSound_0`)))
    (bind _returnvalue (`GameplayStatics.SpawnSound2D` (`self.Sound`) 2.0 1.0 0.0 null))
    (set `self.ShopSound_0` _returnvalue)))

(event `self.Box.OnComponentEndOverlap`
  (params (OverlappedComponent :type "PrimitiveComponent Object Reference") (OtherActor :type "Actor Object Reference") (OtherComp :type "PrimitiveComponent Object Reference") (OtherBodyIndex :type Integer))
  (bind _shopsound_0 (`self.ShopSound_0`))
  (`self.HandleShopExit` OtherActor)
  (cast `/Game/VRTemplate/Blueprints/VRPawn` OtherActor)
  (if (`AudioComponent.IsPlaying` _shopsound_0)
    (`AudioComponent.AdjustVolume` _shopsound_0 0.0 0.0 "Linear")
    (`AudioComponent.SetVolumeMultiplier` _shopsound_0 0.0)
    (`AudioComponent.Stop` _shopsound_0)))

(fn `UserConstructionScript`)