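; Pressure plate button that runs console commands when actors step on and off it, with optional text showing the enter command.
; Tracks overlapping actors so only the first entry and last exit play or reverse the Press timeline, which lerps the dynamic material's emissive to green.
; When the timeline finishes, its direction selects ButtonEnabled or ButtonDisabled, firing the enter command or, on release, either a separate exit command or the same one.
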(event `self.Trigger.OnComponentBeginOverlap`
  (params (OverlappedComponent :type "PrimitiveComponent Object Reference") (OtherActor :type "Actor Object Reference") (OtherComp :type "PrimitiveComponent Object Reference") (OtherBodyIndex :type Integer) (bFromSweep :type Boolean) (SweepResult :type "HitResult Structure (by ref)"))
  ; Check and store overlapping actors on the plate. Saving a list of actors so that the plate only toggles off when all actors are removed.
  (if (`KismetArrayLibrary.Array_IsEmpty` (`self.OverlappedActors`))
    (`KismetArrayLibrary.Array_Add` (`self.OverlappedActors`) OtherActor) ; Add overlapping actor to an array and continue logic
    (bind (_direction _glow) (`Timeline|Press` :!label _label) ; Timeline for animating the button press
      (:`Update`
        ; Update button Visuals using Floats driven by the Timeline
        (`MaterialInstanceDynamic.SetVectorParameterValue` (`self.Button material`) "Emissive" (`KismetMathLibrary.LinearColorLerp` (`self.DefaultEmissiveValue`) (struct :`G` 1.0 :`A` 1.0) _glow)) ; Change emissive color of the button
      )
      (:`Finished`
        ; Trigger a Blueprint Interface when the switch has finished animating.
        (if (`|EnumEquality` _direction "Forward")
          (`self.ButtonEnabled`) ; Calls Button State - These calls will fire logic in child classes
          (else
            (`self.ButtonDisabled`)))))
    (else
      (`KismetArrayLibrary.Array_Add` (`self.OverlappedActors`) OtherActor) ; Add overlapping actor to an array. Not the first item so don't fire execs
    )))

(event `self.Trigger.OnComponentEndOverlap`
  (params (OverlappedComponent :type "PrimitiveComponent Object Reference") (OtherActor :type "Actor Object Reference") (OtherComp :type "PrimitiveComponent Object Reference") (OtherBodyIndex :type Integer))
  ; Check and store overlapping actors on the plate. Saving a list of actors so that the plate only toggles off when all actors are removed.
  (`KismetArrayLibrary.Array_RemoveItem` (`self.OverlappedActors`) OtherActor) ; Remove actor from list
  (if (`KismetArrayLibrary.Array_IsEmpty` (`self.OverlappedActors`))
    (goto _label :!via `Reverse`)))

(event `ButtonEnabled`
  ; Execute Console Command on Enter
  (`KismetSystemLibrary.ExecuteConsoleCommand` (`self.EnterCommand`) null))

(event `ButtonDisabled`
  ; Execute Console Command on Exit. Support for a toggling the same or a new command.
  (`KismetSystemLibrary.ExecuteConsoleCommand` (`KismetMathLibrary.SelectString` (`self.ExitCommand`) (`self.EnterCommand`) (`self.UseExitCommand?`)) null))

(fn `UserConstructionScript`
  (bind _showcommandtext (`self.ShowCommandText`))
  (bind _consoletext (`self.ConsoleText`))
  (bind _returnvalue (`PrimitiveComponent.CreateDynamicMaterialInstance` (`self.Button base`) 1 null "None")) ; Make and apply a dynamic material instance for the button
  (bind _output_get (set `self.Button material` _returnvalue)) ; Set the material as a variable for animating
  (bind _returnvalue_2 (`MaterialInstanceDynamic.K2_GetVectorParameterValue` _output_get "Emissive")) ; Return the Parameter 'Emissive' from the dynamic material
  (set `self.DefaultEmissiveValue` _returnvalue_2) ; Store the default value. Used for lerping between the original and a new color.
  ; Setup Text
  (`SceneComponent.SetVisibility` (`self.Scene`) _showcommandtext true) ; Show or Hide the Text based on setting
  (if _showcommandtext
    (`TextRenderComponent.K2_SetText` _consoletext (`|FormatText` "'{Command}'" (`self.EnterCommand`))) ; Set text to the command to be fired on enter
    (`TextRenderComponent.SetWorldSize` _consoletext (`self.TextSize`)) ; Set text size
    (`TextRenderComponent.SetTextRenderColor` _consoletext (`self.TextColor`))
    (`TextRenderComponent.SetTextRenderColor` (`self.Title`) (`self.TextColor`))))